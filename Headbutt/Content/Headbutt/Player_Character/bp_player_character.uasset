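; Player character blueprint that swaps its skeletal mesh between two lane positions on left/right input and tracks score and lives.
; Tick increments a frame counter that raises a stepped score multiplier, while a looping timer deducts a life and adds multiplied payout.
; Results go to a viewport HUD and a widget component, with score also broadcast to widgets through an interface.
; The game-over pause logic is disconnected.
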(event `EnhancedInput|/Game/Headbutt/Player_Character/IA_Right`
  (params (ActionValue :type Boolean) (ElapsedSeconds :type "Float (double-precision)") (TriggeredSeconds :type "Float (double-precision)") (InputAction :type "InputAction Object Reference" :default "/Game/Headbutt/Player_Character/IA_Right.IA_Right"))
  (:`Triggered`
    (`SceneComponent.K2_SetWorldLocation` (`self.SkeletalMesh`) (`self.left_lane`) true false)))

(event `EnhancedInput|/Game/Headbutt/Player_Character/IA_Left`
  (params (ActionValue :type Boolean) (ElapsedSeconds :type "Float (double-precision)") (TriggeredSeconds :type "Float (double-precision)") (InputAction :type "InputAction Object Reference" :default "/Game/Headbutt/Player_Character/IA_Left.IA_Left"))
  (:`Triggered`
    (`SceneComponent.K2_SetWorldLocation` (`self.SkeletalMesh`) (`self.Right_lane`) true false)))

(event `self.ReceiveTick`
  (params (DeltaSeconds :type "Float (single-precision)"))
  (`self.Calculate multiplier`))

(event `self.ReceiveBeginPlay`
  (`self.Update_Score`)
  (`KismetSystemLibrary.K2_SetTimerDelegate` (delegate `CustomEvent`) 2.0 true)
  (bind _returnvalue (`|CreateWidget` "/Game/Headbutt/UI/WB_HUD.WB_HUD_C"))
  (bind _output_get (set `self.HUD` _returnvalue))
  (`UserWidget.AddToViewport` _output_get 0))

(event `CustomEvent`
  (`self.Take_Damage`)
  (`self.Update_Score`))

(fn `Calculate multiplier`
  (bind _timer (`self.timer`))
  (bind _timer_2 (`self.timer`))
  (bind _timer_3 (`self.timer`))
  (bind _timer_4 (`self.timer`))
  (bind _timer_5 (`self.timer`))
  (bind _timer_6 (`self.timer`))
  (bind _timer_7 (`self.timer`))
  (set `self.timer` (+ (`self.timer`) 1))
  (if (and (> _timer_2 0) (<= _timer_2 100))
    (bind _output_get (set `self.Multiplier` 1.0))
    (elif (and (> _timer_3 100) (<= _timer_3 200))
      (bind _output_get_2 (set `self.Multiplier` 1.5))
      (elif (and (> _timer_4 200) (<= _timer_4 300))
        (bind _output_get_3 (set `self.Multiplier` 2.0))
        (elif (and (> _timer_5 300) (<= _timer_5 400))
          (bind _output_get_4 (set `self.Multiplier` 3.0))
          (elif (and (> _timer_6 400) (<= _timer_6 500))
            (bind _output_get_5 (set `self.Multiplier` 4.0))
            (elif (and (> _timer_7 500) (<= _timer_7 550))
              (bind _output_get_6 (set `self.Multiplier` 6.0))
              (elif (and (> _timer 550) (<= _timer 600))
                (bind _output_get_7 (set `self.Multiplier` 7.0))
                (elif (> (`self.timer`) 600)
                  (bind _output_get_8 (set `self.Multiplier` 8.0)))))))))))

(fn `SetScoreText`
  (params (Multiplier :type "Float (double-precision)"))
  ; Every widget with this interface does the same thing
  (bind _foundwidgets (`WidgetBlueprintLibrary.GetAllWidgetsWithInterface` "/Game/Headbutt/BPI_.BPI__C"))
  (for _array_element _foundwidgets
    (message `/Game/Headbutt/BPI_.Scoreupdate` _array_element Multiplier)))

(fn `Take_Damage`
  (bind _hud (`self.HUD`))
  (bind _output_get (set `self.Lives` (- (`self.Lives`) 1)))
  (`KismetSystemLibrary.PrintString` (`KismetStringLibrary.Conv_IntToString` _output_get))
  (`/Engine/EditorBlueprintResources/StandardMacros.IsValid` _hud
    (:`Is Valid`
      (`/Game/Headbutt/UI/WB_HUD.TakeDamageHUD` _hud _output_get)
      (bind _aswb_hud (cast `/Game/Headbutt/UI/WB_HUD` (`WidgetComponent.GetWidget` (`/Game/Headbutt/UI/BP_Score_Widget.Widget` (`self.Scorewidget`)))))
      (`/Game/Headbutt/UI/WB_HUD.TakeDamageHUD` _aswb_hud _output_get)
      (if (< (`self.Lives`) 1)
        (if (`KismetMathLibrary.Conv_IntToBool` (`self.timer`))
          _)))))

(fn `Update_Score`
  (bind _hud (`self.HUD`))
  (bind _raw_score (`self.raw_score`))
  (bind _returnvalue (* (`self.Payout`) (`self.Multiplier`)))
  (`KismetSystemLibrary.PrintString` (`KismetStringLibrary.Conv_DoubleToString` _raw_score))
  (set `self.Score_Added` _returnvalue)
  (bind _output_get (set `self.raw_score` (+ _returnvalue _raw_score)))
  (`self.SetScoreText` _raw_score)
  (bind _output_get_2 (set `self.score` (`KismetMathLibrary.FTrunc` _output_get)))
  (`/Engine/EditorBlueprintResources/StandardMacros.IsValid` _hud
    (:`Is Valid`
      (`/Game/Headbutt/UI/WB_HUD.ScoreHUDUpdate` _hud _output_get_2)
      (bind _aswb_hud (cast `/Game/Headbutt/UI/WB_HUD` (`WidgetComponent.GetWidget` (`/Game/Headbutt/UI/BP_Score_Widget.Widget` (`self.Scorewidget`)))))
      (`/Game/Headbutt/UI/WB_HUD.ScoreHUDUpdate` _aswb_hud _output_get_2))))

(fn `UserConstructionScript`)