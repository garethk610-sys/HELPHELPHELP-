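; Player character Blueprint for Headbutt that tracks score, score multiplier, lives and game-over state.
; Every Tick increments a frame-based timer, which raises the multiplier in fixed steps up to a cap, with no reset here.
; UpdateScore adds payout times multiplier to a raw total and prints the truncated score.
; TakeDamage removes and prints a life, pausing the game and setting GameOver when none remain.
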(event `self.ReceiveTick`
  (params (DeltaSeconds :type "Float (single-precision)"))
  (`self.Calculate multiplier`))

(fn `Calculate multiplier`
  (bind _timer (`self.timer`))
  (bind _timer_2 (`self.timer`))
  (bind _timer_3 (`self.timer`))
  (bind _timer_4 (`self.timer`))
  (bind _timer_5 (`self.timer`))
  (bind _timer_6 (`self.timer`))
  (bind _timer_7 (`self.timer`))
  (set `self.timer` (+ (`self.timer`) 1))
  (if (and (> _timer_2 0) (<= _timer_2 100))
    (set `self.Multiplier` 1.0)
    (elif (and (> _timer_3 100) (<= _timer_3 200))
      (set `self.Multiplier` 1.5)
      (elif (and (> _timer_4 200) (<= _timer_4 300))
        (set `self.Multiplier` 2.0)
        (elif (and (> _timer_5 300) (<= _timer_5 400))
          (set `self.Multiplier` 3.0)
          (elif (and (> _timer_6 400) (<= _timer_6 500))
            (set `self.Multiplier` 4.0)
            (elif (and (> _timer_7 500) (<= _timer_7 550))
              (set `self.Multiplier` 6.0)
              (elif (and (> _timer 550) (<= _timer 600))
                (set `self.Multiplier` 7.0)
                (elif (> (`self.timer`) 600)
                  (set `self.Multiplier` 8.0))))))))))

(fn `Take_Damage`
  (bind _output_get (set `self.Lives` (- (`self.Lives`) 1)))
  (`KismetSystemLibrary.PrintString` (`KismetStringLibrary.Conv_IntToString` _output_get))
  (if (< (`self.Lives`) 1)
    (`GameplayStatics.SetGamePaused` true)
    (set `self.game_over` true)))

(fn `Update_Score`
  (bind _output_get (set `self.raw_score` (+ (* (`self.Payout`) (`self.Multiplier`)) (`self.raw_score`))))
  (bind _output_get_2 (set `self.score` (`KismetMathLibrary.FTrunc` _output_get)))
  (`KismetSystemLibrary.PrintString` (`KismetStringLibrary.Conv_IntToString` _output_get_2)))

(fn `UserConstructionScript`)