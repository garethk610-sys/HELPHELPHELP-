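; Spawner for the Headbutt game that launches balloons (less often) or boulders from three spawn points with a negative-Y impulse.
; BeginPlay caches the three Spawner transforms, with component numbers shifted relative to the variable names.
; Each Tick randomly picks one of six patterns, three single-point and three paired.
; Each pattern has its own random Delay, which ignores re-triggers while pending, so the patterns run as overlapping timers.
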(event `self.ReceiveBeginPlay`
  (set `self.Spawner1Location` (`SceneComponent.K2_GetComponentToWorld` (`self.spawner3`)))
  (set `self.Spawner2Location` (`SceneComponent.K2_GetComponentToWorld` (`self.spawner1`)))
  (set `self.Spawner3Location` (`SceneComponent.K2_GetComponentToWorld` (`self.spawner2`))))

(event `self.ReceiveTick`
  (params (DeltaSeconds :type "Float (single-precision)"))
  (bind _spawner1location (`self.Spawner1Location`))
  (bind _spawner1location_2 (`self.Spawner1Location`))
  (bind _spawner2location (`self.Spawner2Location`))
  (bind _spawner3location (`self.Spawner3Location`))
  (bind _spawner2location_2 (`self.Spawner2Location`))
  (bind _spawner1location_3 (`self.Spawner1Location`))
  (bind _spawner3location_2 (`self.Spawner3Location`))
  (bind _spawner2location_3 (`self.Spawner2Location`))
  (bind _spawner3location_3 (`self.Spawner3Location`))
  (set `self.SpawnLocationChooser` (`KismetMathLibrary.RandomIntegerInRange` 1 6))
  (if (== (`self.SpawnLocationChooser`) 1)
    (set `self.spawnitemchooser` (`KismetMathLibrary.RandomIntegerInRange` 1 5))
    (`KismetSystemLibrary.Delay` (`KismetMathLibrary.Conv_IntToDouble` (`KismetMathLibrary.RandomIntegerInRange` 5 10)))
    (bind _output_get (set `self.spawntracker_bool` (< (`self.spawnitemchooser`) 2)))
    (if _output_get
      (bind _returnvalue (`|SpawnActorFromClass` "/Game/Headbutt/bp_balloon.bp_balloon_C" _spawner1location "Undefined" "MultiplyWithRoot" null null))
      (`KismetSystemLibrary.PrintString` "balloon")
      (`PrimitiveComponent.AddImpulse` (`/Game/Headbutt/bp_balloon.balloon` _returnvalue) (0.0 -80.0 0.0) "None" false)
      (else
        (bind _returnvalue_2 (`|SpawnActorFromClass` "/Game/Headbutt/bp_boulder.bp_boulder_C" _spawner1location "Undefined" "MultiplyWithRoot" null null))
        (`KismetSystemLibrary.PrintString` "boulder")
        (`PrimitiveComponent.AddImpulse` (`/Game/Headbutt/bp_boulder.boulder` _returnvalue_2) (0.0 -100.0 0.0) "None" false)))
    (elif (== (`self.SpawnLocationChooser`) 2)
      (set `self.spawnitemchooser` (`KismetMathLibrary.RandomIntegerInRange` 1 5))
      (`KismetSystemLibrary.Delay` (`KismetMathLibrary.Conv_IntToDouble` (`KismetMathLibrary.RandomIntegerInRange` 1 3)))
      (bind _output_get_2 (set `self.spawntracker_bool` (< (`self.spawnitemchooser`) 2)))
      (if _output_get_2
        (bind _returnvalue_3 (`|SpawnActorFromClass` "/Game/Headbutt/bp_balloon.bp_balloon_C" _spawner2location "Undefined" "MultiplyWithRoot" null null))
        (`KismetSystemLibrary.PrintString` "balloon")
        (`PrimitiveComponent.AddImpulse` (`/Game/Headbutt/bp_balloon.balloon` _returnvalue_3) (0.0 -80.0 0.0) "None" false)
        (else
          (bind _returnvalue_4 (`|SpawnActorFromClass` "/Game/Headbutt/bp_boulder.bp_boulder_C" _spawner2location "Undefined" "MultiplyWithRoot" null null))
          (`KismetSystemLibrary.PrintString` "boulder")
          (`PrimitiveComponent.AddImpulse` (`/Game/Headbutt/bp_boulder.boulder` _returnvalue_4) (0.0 -100.0 0.0) "None" false)))
      (elif (== (`self.SpawnLocationChooser`) 3)
        (set `self.spawnitemchooser` (`KismetMathLibrary.RandomIntegerInRange` 1 5))
        (`KismetSystemLibrary.Delay` (`KismetMathLibrary.Conv_IntToDouble` (`KismetMathLibrary.RandomIntegerInRange` 1 3)))
        (bind _output_get_3 (set `self.spawntracker_bool` (< (`self.spawnitemchooser`) 2)))
        (if _output_get_3
          (bind _returnvalue_5 (`|SpawnActorFromClass` "/Game/Headbutt/bp_balloon.bp_balloon_C" _spawner3location "Undefined" "MultiplyWithRoot" null null))
          (`KismetSystemLibrary.PrintString` "balloon")
          (`PrimitiveComponent.AddImpulse` (`/Game/Headbutt/bp_balloon.balloon` _returnvalue_5) (0.0 -80.0 0.0) "None" false)
          (else
            (bind _returnvalue_6 (`|SpawnActorFromClass` "/Game/Headbutt/bp_boulder.bp_boulder_C" _spawner3location "Undefined" "MultiplyWithRoot" null null))
            (`KismetSystemLibrary.PrintString` "boulder")
            (`PrimitiveComponent.AddImpulse` (`/Game/Headbutt/bp_boulder.boulder` _returnvalue_6) (0.0 -100.0 0.0) "None" false)))
        (elif (== (`self.SpawnLocationChooser`) 4)
          (set `self.spawnitemchooser` (`KismetMathLibrary.RandomIntegerInRange` 1 5))
          (`KismetSystemLibrary.Delay` (`KismetMathLibrary.Conv_IntToDouble` (`KismetMathLibrary.RandomIntegerInRange` 1 3)))
          (bind _output_get_4 (set `self.spawntracker_bool` (< (`self.spawnitemchooser`) 2)))
          (if _output_get_4
            (bind _returnvalue_7 (`|SpawnActorFromClass` "/Game/Headbutt/bp_balloon.bp_balloon_C" _spawner1location_2 "Undefined" "MultiplyWithRoot" null null))
            (`KismetSystemLibrary.PrintString` "balloon")
            (`PrimitiveComponent.AddImpulse` (`/Game/Headbutt/bp_balloon.balloon` _returnvalue_7) (0.0 -80.0 0.0) "None" false)
            (bind _returnvalue_8 (`|SpawnActorFromClass` "/Game/Headbutt/bp_balloon.bp_balloon_C" _spawner2location_2 "Undefined" "MultiplyWithRoot" null null))
            (`KismetSystemLibrary.PrintString` "balloon")
            (`PrimitiveComponent.AddImpulse` (`/Game/Headbutt/bp_balloon.balloon` _returnvalue_8) (0.0 -80.0 0.0) "None" false)
            (else
              (bind _returnvalue_9 (`|SpawnActorFromClass` "/Game/Headbutt/bp_boulder.bp_boulder_C" _spawner1location_2 "Undefined" "MultiplyWithRoot" null null))
              (`KismetSystemLibrary.PrintString` "boulder")
              (`PrimitiveComponent.AddImpulse` (`/Game/Headbutt/bp_boulder.boulder` _returnvalue_9) (0.0 -100.0 0.0) "None" false)
              (bind _returnvalue_10 (`|SpawnActorFromClass` "/Game/Headbutt/bp_boulder.bp_boulder_C" _spawner2location_2 "Undefined" "MultiplyWithRoot" null null))
              (`KismetSystemLibrary.PrintString` "boulder")
              (`PrimitiveComponent.AddImpulse` (`/Game/Headbutt/bp_boulder.boulder` _returnvalue_10) (0.0 -100.0 0.0) "None" false)))
          (elif (== (`self.SpawnLocationChooser`) 5)
            (set `self.spawnitemchooser` (`KismetMathLibrary.RandomIntegerInRange` 1 5))
            (`KismetSystemLibrary.Delay` (`KismetMathLibrary.Conv_IntToDouble` (`KismetMathLibrary.RandomIntegerInRange` 1 3)))
            (bind _output_get_5 (set `self.spawntracker_bool` (< (`self.spawnitemchooser`) 2)))
            (if _output_get_5
              (bind _returnvalue_11 (`|SpawnActorFromClass` "/Game/Headbutt/bp_balloon.bp_balloon_C" _spawner1location_3 "Undefined" "MultiplyWithRoot" null null))
              (`KismetSystemLibrary.PrintString` "balloon")
              (`PrimitiveComponent.AddImpulse` (`/Game/Headbutt/bp_balloon.balloon` _returnvalue_11) (0.0 -80.0 0.0) "None" false)
              (bind _returnvalue_12 (`|SpawnActorFromClass` "/Game/Headbutt/bp_balloon.bp_balloon_C" _spawner3location_2 "Undefined" "MultiplyWithRoot" null null))
              (`KismetSystemLibrary.PrintString` "balloon")
              (`PrimitiveComponent.AddImpulse` (`/Game/Headbutt/bp_balloon.balloon` _returnvalue_12) (0.0 -80.0 0.0) "None" false)
              (else
                (bind _returnvalue_13 (`|SpawnActorFromClass` "/Game/Headbutt/bp_boulder.bp_boulder_C" _spawner1location_3 "Undefined" "MultiplyWithRoot" null null))
                (`KismetSystemLibrary.PrintString` "boulder")
                (`PrimitiveComponent.AddImpulse` (`/Game/Headbutt/bp_boulder.boulder` _returnvalue_13) (0.0 -100.0 0.0) "None" false)
                (bind _returnvalue_14 (`|SpawnActorFromClass` "/Game/Headbutt/bp_boulder.bp_boulder_C" _spawner3location_2 "Undefined" "MultiplyWithRoot" null null))
                (`KismetSystemLibrary.PrintString` "boulder")
                (`PrimitiveComponent.AddImpulse` (`/Game/Headbutt/bp_boulder.boulder` _returnvalue_14) (0.0 -100.0 0.0) "None" false)))
            (elif (== (`self.SpawnLocationChooser`) 6)
              (set `self.spawnitemchooser` (`KismetMathLibrary.RandomIntegerInRange` 1 5))
              (`KismetSystemLibrary.Delay` (`KismetMathLibrary.Conv_IntToDouble` (`KismetMathLibrary.RandomIntegerInRange` 1 3)))
              (bind _output_get_6 (set `self.spawntracker_bool` (< (`self.spawnitemchooser`) 2)))
              (if _output_get_6
                (bind _returnvalue_15 (`|SpawnActorFromClass` "/Game/Headbutt/bp_balloon.bp_balloon_C" _spawner2location_3 "Undefined" "MultiplyWithRoot" null null))
                (`KismetSystemLibrary.PrintString` "balloon")
                (`PrimitiveComponent.AddImpulse` (`/Game/Headbutt/bp_balloon.balloon` _returnvalue_15) (0.0 -80.0 0.0) "None" false)
                (bind _returnvalue_16 (`|SpawnActorFromClass` "/Game/Headbutt/bp_balloon.bp_balloon_C" _spawner3location_3 "Undefined" "MultiplyWithRoot" null null))
                (`KismetSystemLibrary.PrintString` "balloon")
                (`PrimitiveComponent.AddImpulse` (`/Game/Headbutt/bp_balloon.balloon` _returnvalue_16) (0.0 -80.0 0.0) "None" false)
                (else
                  (bind _returnvalue_17 (`|SpawnActorFromClass` "/Game/Headbutt/bp_boulder.bp_boulder_C" _spawner2location_3 "Undefined" "MultiplyWithRoot" null null))
                  (`KismetSystemLibrary.PrintString` "boulder")
                  (`PrimitiveComponent.AddImpulse` (`/Game/Headbutt/bp_boulder.boulder` _returnvalue_17) (0.0 -100.0 0.0) "None" false)
                  (bind _returnvalue_18 (`|SpawnActorFromClass` "/Game/Headbutt/bp_boulder.bp_boulder_C" _spawner3location_3 "Undefined" "MultiplyWithRoot" null null))
                  (`KismetSystemLibrary.PrintString` "boulder")
                  (`PrimitiveComponent.AddImpulse` (`/Game/Headbutt/bp_boulder.boulder` _returnvalue_18) (0.0 -100.0 0.0) "None" false))))))))))

(fn `UserConstructionScript`)