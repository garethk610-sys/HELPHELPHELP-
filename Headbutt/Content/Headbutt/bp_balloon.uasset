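; Balloon target in the Headbutt game that awards score when the player pawn touches it.
; Overlap on the Balloon component casts to BP_Player_Pawn and calls UpdateScore, leaving the balloon in place.
; A separate SelfDestruct function, not called here, spawns BP_Scoreactor at the balloon, updates BP_XRPawn's score and destroys the actor.
; The actor-level overlap and Scoreupdate events do nothing further.
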(event `self.ReceiveActorBeginOverlap`
  (params (OtherActor :type "Actor Object Reference"))
  (cast `/Game/Headbutt/Player_Character/BP_Player_Pawn` OtherActor))

(event `/Game/Headbutt/UI/BPI_.Scoreupdate`
  (params (Multiplier :type "Float (double-precision)")))

(event `self.balloon.OnComponentBeginOverlap`
  (params (OverlappedComponent :type "PrimitiveComponent Object Reference") (OtherActor :type "Actor Object Reference") (OtherComp :type "PrimitiveComponent Object Reference") (OtherBodyIndex :type Integer) (bFromSweep :type Boolean) (SweepResult :type "HitResult Structure (by ref)"))
  (bind _asbp_player_pawn (cast `/Game/Headbutt/Player_Character/BP_Player_Pawn` OtherActor))
  (`/Game/Headbutt/Player_Character/BP_Player_Pawn.Update_Score` _asbp_player_pawn))

(fn `Self_Destruct`
  ; Spawn Number when balloon self destructs
  (`KismetSystemLibrary.PrintString` "update")
  (`|SpawnActorFromClass` "/Game/Headbutt/UI/Actors/BP_Scoreactor.BP_Scoreactor_C" (`KismetMathLibrary.MakeTransform` (`SceneComponent.K2_GetComponentLocation` (`self.balloon`))) "Undefined" "MultiplyWithRoot" null null)
  (bind _asbp_xrpawn (cast `/Game/XRFramework/Blueprints/BP_XRPawn` (`GameplayStatics.GetPlayerPawn` 0)))
  (`/Game/XRFramework/Blueprints/BP_XRPawn.Update_Score` _asbp_xrpawn)
  (`self.K2_DestroyActor`))

(fn `UserConstructionScript`)